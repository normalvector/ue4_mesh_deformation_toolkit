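; SaveToSMTest_BP is a test Blueprint for saving deformed geometry to a static mesh with a MeshDeformation component.
; Its construction script loads MaterialBall, selects vertices near a center with inner and outer radii, eases the selection, and translates it by Delta.
; The result saves to SaveTarget using the ProceduralMesh component and two plastic materials.
; A direct save to the procedural mesh is left unconnected, and the event graph is inactive.
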(event EventBeginPlay)

(event Collision|EventActorBeginOverlap
  (params (OtherActor :type Actor%20Object%20Reference)))

(event EventTick
  (params (DeltaSeconds :type Float%20%28single-precision%29)))

(fn ConstructionScript
  (bind _meshdeformationcomponent (Class|MeshDeformationComponent|LoadfromStaticMesh (Variables|Default|GetMeshDeformation) "/Game/MDT/Demo/DeformTestMeshes/MaterialBall.MaterialBall"))
  (bind _meshdeformationcomponent_2 (Class|MeshDeformationComponent|Translate _meshdeformationcomponent (Variables|Default|GetDelta) (Class|SelectionSetBPLibrary|Ease (Class|MeshDeformationComponent|SelectNear _meshdeformationcomponent (Variables|Default|GetCenter) (Variables|Default|GetInnerRadius) (Variables|Default|GetOuterRadius)) "EaseInOut" 2 2.0)))
  (Class|MeshDeformationComponent|SavetoStaticMesh _meshdeformationcomponent_2 "/Game/MDT/Test/SaveTarget.SaveTarget" (Variables|Default|GetProceduralMesh) (Utilities|Array|MakeArray "/Game/MDT/Demo/Materials/SimplePBR/MI_ShinyPlasticOrange.MI_ShinyPlasticOrange" "/Game/MDT/Demo/Materials/SimplePBR/MI_ShinyPlasticWhite.MI_ShinyPlasticWhite")))