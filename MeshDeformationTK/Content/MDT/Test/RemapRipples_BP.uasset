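; RemapRipples_BP is a test Blueprint that deforms a plane mesh into ripples using the MeshDeformation component.
; The construction script loads a dense static plane and selects vertices by radial falloff around the origin.
; RemapRipple reshapes that selection using the ripple count and up-and-down settings, which weights a vertical translation.
; The result is saved to a procedural mesh without collision, with no active runtime logic.
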(event EventBeginPlay)

(event Collision|EventActorBeginOverlap
  (params (OtherActor :type Actor%20Object%20Reference)))

(event EventTick
  (params (DeltaSeconds :type Float%20%28single-precision%29)))

(fn ConstructionScript
  (bind _meshdeformationcomponent (Class|MeshDeformationComponent|LoadfromStaticMesh (Variables|Default|GetMeshDeformation) "/Game/MDT/Demo/DeformTestMeshes/Plane_128x128.Plane_128x128"))
  (bind _meshdeformationcomponent_2 (Class|MeshDeformationComponent|Translate _meshdeformationcomponent "0, 0,50.000000" (Class|SelectionSetBPLibrary|RemapRipple (Class|MeshDeformationComponent|SelectNear _meshdeformationcomponent "0, 0, 0" 1e+01 45.0) (Variables|Default|GetNumberOfRipples) (Variables|Default|GetUpAndDown))))
  (Class|MeshDeformationComponent|SavetoProceduralMeshComponent _meshdeformationcomponent_2 (Variables|Default|GetProceduralMesh) false))