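; Test Blueprint for a tiling landscape piece, built in the construction script with MeshDeformation.
; It loads a static mesh and raises its vertices along Z, weighted by a Perlin fractal noise selection.
; The actor's transform drives the noise translation, rotation and scale, so the relief follows the piece's placement.
; The result is saved to a procedural mesh without collision, then given the materials from an array.
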(event EventBeginPlay)

(event Collision|EventActorBeginOverlap
  (params (OtherActor :type Actor%20Object%20Reference)))

(event EventTick
  (params (DeltaSeconds :type Float%20%28single-precision%29)))

(fn ConstructionScript
  (bind _returnvalue (Transformation|GetActorTransform))
  (bind (_location _rotation _scale) (Math|Transform|BreakTransform _returnvalue))
  (bind _meshdeformationcomponent (Class|MeshDeformationComponent|LoadfromStaticMesh (Variables|Default|GetMeshDeformation) (Variables|Default|GetStaticMesh)))
  (bind _meshdeformationcomponent_2 (Class|MeshDeformationComponent|Translate _meshdeformationcomponent "0, 0,50.000000" (Class|MeshDeformationComponent|SelectbyNoise _meshdeformationcomponent 1337 0.01 "Quintic" "PerlinFractal" 3 2.0 0.5 "FBM" "Euclidian" _location _rotation _scale)))
  (Class|MeshDeformationComponent|SavetoProceduralMeshComponent _meshdeformationcomponent_2 (Variables|Default|GetProceduralMesh) false)
  (for (_array_element _array_index) (Variables|Default|GetMaterials)
    (Rendering|Material|SetMaterial (Variables|Default|GetProceduralMesh) _array_index _array_element)))