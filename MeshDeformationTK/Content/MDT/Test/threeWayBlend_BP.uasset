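; Test Blueprint that builds a noise-displaced plane in its construction script using mesh deformation selection sets.
; A 128x128 plane is loaded, translated upward by a blended selection, then saved to a procedural mesh without collision.
; The selection lerps between remapped Perlin fractal and cellular noise, using an eased, inverted radial falloff around the origin as per-vertex alpha.
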(event EventBeginPlay)

(event Collision|EventActorBeginOverlap
  (params (OtherActor :type Actor%20Object%20Reference)))

(event EventTick
  (params (DeltaSeconds :type Float%20%28single-precision%29)))

(fn ConstructionScript
  (bind _meshdeformationcomponent (Class|MeshDeformationComponent|LoadfromStaticMesh (Variables|Default|GetMeshDeformation) "/Game/MDT/Demo/DeformTestMeshes/Plane_128x128.Plane_128x128"))
  (bind _meshdeformationcomponent_2 (Class|MeshDeformationComponent|Translate _meshdeformationcomponent "0.000000, 0,25.000000" (Class|SelectionSetBPLibrary|LerpSelectionSetswithSelectionSet (Class|SelectionSetBPLibrary|RemaptoRange (Class|MeshDeformationComponent|SelectbyNoise :self (Variables|Default|GetMeshDeformation) :NoiseType "PerlinFractal") 0.0 1.0) (Class|SelectionSetBPLibrary|RemaptoRange (Class|MeshDeformationComponent|SelectbyNoise :self (Variables|Default|GetMeshDeformation) :Frequency 0.1 :NoiseType "Cellular") 0.0 1.0) (Class|SelectionSetBPLibrary|OneMinus (Class|SelectionSetBPLibrary|Ease (Class|MeshDeformationComponent|SelectNear (Variables|Default|GetMeshDeformation) "0, 0, 0" 2e+01 4e+01) "EaseInOut" 2 2.0)))))
  (Class|MeshDeformationComponent|SavetoProceduralMeshComponent _meshdeformationcomponent_2 (Variables|Default|GetProceduralMesh) false))