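; SplineTest_BP is a test Blueprint for the mesh deformation component, bending a static mesh along a spline.
; The construction script loads LOD 0 of the mesh into MeshDeformation and fits its geometry to the Spline between configurable start and end positions.
; The result is saved to a procedural mesh without collision and given an orange plastic material.
; BeginPlay is empty, so all work happens at construction.
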(event EventBeginPlay)

(fn ConstructionScript
  (bind _meshdeformationcomponent (Class|MeshDeformationComponent|LoadfromStaticMesh (Variables|Default|GetMeshDeformation) (Variables|Default|GetStaticMesh)))
  (Class|MeshGeometry|FittoSpline (Variables|/Script/MeshDeformationToolkit.MeshDeformationComponent|GetMeshGeometry _meshdeformationcomponent) (Variables|Default|GetSpline) (Variables|Default|GetStartPosition) (Variables|Default|GetEndPosition) 1.0)
  (Class|MeshDeformationComponent|SavetoProceduralMeshComponent _meshdeformationcomponent (Variables|Default|GetProceduralMesh) false)
  (Rendering|Material|SetMaterial (Variables|Default|GetProceduralMesh) 0 "/Game/MDT/Demo/Materials/SimplePBR/MI_ShinyPlasticOrange.MI_ShinyPlasticOrange"))