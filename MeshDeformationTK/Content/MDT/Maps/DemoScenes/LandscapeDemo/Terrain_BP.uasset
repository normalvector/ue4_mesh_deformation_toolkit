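; Demo terrain actor that procedurally sculpts a low landscape from the Ground static mesh in its Construction Script.
; A MeshDeformation component loads the mesh, carves a riverbed along RivereSpline, adds fractal Perlin noise, and shapes a central mound with a dipped middle.
; Each step is a Translate weighted by selection sets, combining volume, distance and noise masks with easing.
; The result is saved to a ProceduralMesh without collision and given materials.
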(event EventBeginPlay)

(event Collision|EventActorBeginOverlap
  (params (OtherActor :type Actor%20Object%20Reference)))

(event EventTick
  (params (DeltaSeconds :type Float%20%28single-precision%29)))

(fn ConstructionScript
  (bind _meshdeformation (Variables|Default|GetMeshDeformation))
  (bind _returnvalue (Class|MeshDeformationComponent|SelectinVolume _meshdeformation "-500.000000,-500.000000,100.000000" "500.000000,500.000000,-5.000000"))
  (bind _meshdeformationcomponent (Class|MeshDeformationComponent|LoadfromStaticMesh (Variables|Default|GetMeshDeformation) "/Game/MDT/Maps/DemoScenes/LandscapeDemo/Ground.Ground"))
  (Class|MeshDeformationComponent|Translate _meshdeformationcomponent "0, 0,-10.000000" (Class|SelectionSetBPLibrary|Ease (Class|MeshDeformationComponent|SelectNearSpline _meshdeformationcomponent (Variables|Default|GetrivereSpline) 0.0 1e+01) "SinusoidalInOut" 2 2.0))
  (bind _meshdeformationcomponent_2 (Class|MeshDeformationComponent|Translate (Variables|Default|GetMeshDeformation) "0.000000,0.000000,2.000000" (Class|SelectionSetBPLibrary|MultiplySelectionSets _returnvalue (Class|SelectionSetBPLibrary|RemaptoRange (Class|MeshDeformationComponent|SelectbyNoise :self _meshdeformation :Frequency 0.1 :NoiseType "PerlinFractal" :FractalOctaves 5) 0.0 1.0))))
  (bind _meshdeformationcomponent_3 (Class|MeshDeformationComponent|Translate _meshdeformationcomponent_2 "0.000000,0.000000,-10.000000" (Class|SelectionSetBPLibrary|MultiplySelectionSets _returnvalue (Class|SelectionSetBPLibrary|Ease (Class|MeshDeformationComponent|SelectNear _meshdeformation "0, 0, 0" 0.0 15.0) "EaseInOut" 2 2.0))))
  (bind _meshdeformationcomponent_4 (Class|MeshDeformationComponent|Translate _meshdeformationcomponent_2 "0.000000,0.000000,10.000000" (Class|SelectionSetBPLibrary|MultiplySelectionSets _returnvalue (Class|SelectionSetBPLibrary|Ease (Class|MeshDeformationComponent|SelectNear _meshdeformation "0, 0, 0" 15.0 4e+01) "EaseIn" 2 2.0))))
  (Class|MeshDeformationComponent|SavetoProceduralMeshComponent _meshdeformationcomponent_4 (Variables|Default|GetProceduralMesh) false)
  (Rendering|Material|SetMaterial (Variables|Default|GetProceduralMesh) 0 0)
  (Rendering|Material|SetMaterial (Variables|Default|GetProceduralMesh) 1 "/Game/MDT/Demo/Materials/LowPolySimplePBR/MI_LowPolyOrangePlastic.MI_LowPolyOrangePlastic"))