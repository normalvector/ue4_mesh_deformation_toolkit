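; Road test Blueprint for a landscape demo that builds a procedural mesh along a spline, conformed to the surface below.
; The construction script loads a 128x128 plane through MeshDeformation and raises a band along its centerline using an eased near-line selection.
; It fits the result to the spline, conforms it downward with a slight height offset, and saves it to a ProceduralMesh component without collision.
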(event EventBeginPlay)

(event Collision|EventActorBeginOverlap
  (params (OtherActor :type Actor%20Object%20Reference)))

(event EventTick
  (params (DeltaSeconds :type Float%20%28single-precision%29)))

(fn ConstructionScript
  (bind _meshdeformationcomponent (Class|MeshDeformationComponent|LoadfromStaticMesh (Variables|Default|GetMeshDeformation) "/Game/MDT/Demo/DeformTestMeshes/Plane_128x128.Plane_128x128"))
  (bind _meshdeformationcomponent_2 (Class|MeshDeformationComponent|Translate _meshdeformationcomponent "0, 0,15.000000" (Class|SelectionSetBPLibrary|Ease (Class|MeshDeformationComponent|SelectNearLine _meshdeformationcomponent "50.000000,0.000000,0.000000" "-50.000000,0.000000,0.000000" 1e+01 5e+01 false true) "SinusoidalInOut" 2 2.0)))
  (bind _meshdeformationcomponent_3 (Class|MeshDeformationComponent|FittoSpline _meshdeformationcomponent_2 (Variables|Default|GetSpline) 0.0 1.0 0.5))
  (bind _meshdeformationcomponent_4 (Class|MeshDeformationComponent|ConformDown _meshdeformationcomponent_3 (Transformation|GetWorldTransform (Variables|Default|GetProceduralMesh)) 0 1e+02 -5.0 true "ECC_WorldStatic"))
  (Class|MeshDeformationComponent|SavetoProceduralMeshComponent _meshdeformationcomponent_4 (Variables|Default|GetProceduralMesh) false)
  (Rendering|Material|SetMaterial (Variables|Default|GetProceduralMesh) 0 "/Game/MDT/Demo/Materials/LowPolySimplePBR/MI_LowPolyWhitePlastic.MI_LowPolyWhitePlastic"))