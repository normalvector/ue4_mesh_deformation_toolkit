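; Test actor that builds a spline-following, conformed girder mesh in its construction script using a MeshDeformation component.
; It loads the Girder static mesh, fits it to the Spline at an enlarged scale, then conforms the geometry using the actor transform and a height offset.
; The result is saved to a procedural mesh with collision and given a shiny orange metal material; the event graph is empty.
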(event EventBeginPlay)

(event Collision|EventActorBeginOverlap
  (params (OtherActor :type Actor%20Object%20Reference)))

(event EventTick
  (params (DeltaSeconds :type Float%20%28single-precision%29)))

(fn ConstructionScript
  (bind _meshdeformationcomponent (Class|MeshDeformationComponent|LoadfromStaticMesh (Variables|Default|GetMeshDeformation) "/Game/Demo/DeformTestMeshes/Girder.Girder"))
  (Class|MeshDeformationComponent|FittoSpline _meshdeformationcomponent (Variables|Default|GetSpline) 0.0 1.0 5.0)
  (Class|MeshGeometry|Conform (Variables|/Script/MeshDeformationToolkit.MeshDeformationComponent|GetMeshGeometry (Variables|Default|GetMeshDeformation)) (Transformation|GetActorTransform) 0 "0.000000,0.000000,-100.000000" 1e+01 true "ECC_WorldStatic")
  (Class|MeshDeformationComponent|SavetoProceduralMeshComponent (Variables|Default|GetMeshDeformation) (Variables|Default|GetProceduralMesh) true)
  (Rendering|Material|SetMaterial (Variables|Default|GetProceduralMesh) 0 "/Game/Demo/Materials/SimplePBR/MI_ShinyMetalOrange.MI_ShinyMetalOrange"))